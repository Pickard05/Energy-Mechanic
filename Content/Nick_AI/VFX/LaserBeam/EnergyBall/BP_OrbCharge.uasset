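; BP_OrbCharge is an energy orb that grows, homes in on the player and briefly slows them.
; On BeginPlay it caches the BP_TheGunPanda player and uses a timeline to scale the orb's Niagara size, emissive and distortion parameters.
; ChargePlayer interpolates the collision box toward the player on a second timeline.
; Any box overlap spawns a shockwave, cuts player walk speed, hides the orb, then restores speed and destroys the actor.
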(event OnComponentBeginOverlap(Box)
  (params (OverlappedComponent :type Primitive%20Component%20Object%20Reference) (OtherActor :type Actor%20Object%20Reference) (OtherComp :type Primitive%20Component%20Object%20Reference) (OtherBodyIndex :type Integer) (bFromSweep :type Boolean) (SweepResult :type Hit%20Result%20Structure%20%28by%20ref%29))
  (bind _as_bp_the_gun_panda (Variables|Default|GetAs%20BP%20The%20Gun%20Panda))
  (bind _charactermovement (Variables|/Script/Engine.Character|GetCharacterMovement _as_bp_the_gun_panda))
  (bind _returnvalue (Niagara|SpawnSystematLocation "/Game/Nick_AI/VFX/Shockwave/NS_Shockwave.NS_Shockwave" (Transformation|GetActorLocation)))
  (Utilities|FlowControl|Delay 0.2)
  (Components|Activation|Deactivate _returnvalue)
  (Variables|/Script/Engine.CharacterMovementComponent|SetMaxWalkSpeed _charactermovement 1.5e+02)
  (Rendering|SetVisibility (Variables|Default|GetOrb) false false)
  (Utilities|FlowControl|Delay 2.0)
  (Variables|/Script/Engine.CharacterMovementComponent|SetMaxWalkSpeed _charactermovement 6e+02)
  (Actor|DestroyActor))

(event Custom|ChargeUP)

(event Custom|CustomEvent)

(event Custom|ChargePlayer
  (bind _trackplayer (Timeline|Timeline Play)
    (:Update
      (Transformation|SetWorldLocation (Variables|Default|GetBox) (Math|Interpolation|VInterpTo (Transformation|GetActorLocation) (Transformation|GetActorLocation (Variables|Default|GetAs%20BP%20The%20Gun%20Panda)) _trackplayer 0.5) false false))))

(event EventBeginPlay
  (Utilities|FlowControl|Sequence
    (:then_0
      (bind _asbp_the_gun_panda (Utilities|Casting|CastToBP_TheGunPanda (Game|GetPlayerCharacter 0)))
      (Variables|Default|SetAs%20BP%20The%20Gun%20Panda _asbp_the_gun_panda))
    (:then_1
      (Utilities|FlowControl|DoOnce false
        (:Completed
          (bind _orbgrowth (Timeline|OrbGrowth PlayFromStart)
            (:Update
              (Effects|Components|ParticleSystem|SetFloatParameter (Variables|Default|GetOrb) "OrbSize" (Math|Float|Lerp 0.0 0.5 _orbgrowth))
              (Effects|Components|ParticleSystem|SetFloatParameter (Variables|Default|GetOrb) "EmissiveSize" (Math|Float|Lerp 0.0 1.0 _orbgrowth))
              (Effects|Components|ParticleSystem|SetFloatParameter (Variables|Default|GetOrb) "InnerOrb" (Math|Float|Lerp 0.0 1.0 _orbgrowth))
              (Effects|Components|ParticleSystem|SetFloatParameter (Variables|Default|GetOrb) "Distortion Size" (Math|Float|Lerp 0.0 0.5 _orbgrowth)))))))))

(fn ConstructionScript)