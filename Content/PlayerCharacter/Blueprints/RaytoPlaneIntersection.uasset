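; Blueprint utility in the player character folder that finds where a ray meets an infinite plane.
; FindRayToPlanePoint uses dot products with the plane normal to get the distance along the ray, then returns the intersection point and a success flag.
; It fails with a zero vector only when the denominator is exactly zero, and does not reject intersections behind the ray origin.
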(fn FindRaytoPlanePoint
  (params (RayOrigin :type Vector) (RayDirection :type Vector) (PlaneNormal :type Vector) (PlanePoint :type Vector))
  (Utilities|FlowControl|Sequence
    (:then_0
      (LocalVariables|SetNumerator (Math|Vector|DotProduct PlaneNormal (- PlanePoint RayOrigin))))
    (:then_1
      (LocalVariables|SetDenominator (Math|Vector|DotProduct PlaneNormal RayDirection)))
    (:then_2
      (if (== (LocalVariables|GetDenominator) 0.0)
        (return false "0, 0, 0")
        (else
          (return true (+ (* (/ (LocalVariables|GetNumerator) (LocalVariables|GetDenominator)) RayDirection) RayOrigin)))))))