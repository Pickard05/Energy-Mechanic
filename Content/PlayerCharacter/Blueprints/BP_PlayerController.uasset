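; Player controller that turns the controlled pawn to face the mouse cursor.
; On BeginPlay it adds the default Enhanced Input mapping context to the local player subsystem.
; Each Tick it deprojects the cursor into a camera ray and intersects it with a horizontal plane at the pawn's location.
; When that hit succeeds, it sets the pawn's yaw toward the intersection point.
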(event EventBeginPlay
  (bind _returnvalue (PlayerController|LocalPlayerSubsystems|GetEnhancedInputLocalPlayerSubsystem))
  (Utilities|IsValid _returnvalue
    (:Is%20Valid
      (Input|AddMappingContext _returnvalue "/Game/TopDown/Input/IMC_Default.IMC_Default" 0 "(bIgnoreAllPressedKeysUntilRelease=True,bForceImmediately=False,bNotifyUserSettings=False)"))))

(event EventTick
  (params (DeltaSeconds :type Float%20%28single-precision%29))
  (bind (_locationx _locationy) (Game|Player|GetMousePosition))
  (bind _returnvalue (Game|GetPlayerCameraManager 0))
  (bind _returnvalue_2 (Pawn|GetControlledPawn))
  (bind _returnvalue_3 (Pawn|GetControlledPawn))
  (bind _self self)
  (bind _worlddirection (Class|GameplayStatics|DeprojectScreentoWorld _self (Math|Vector2D|MakeVector2D _locationx _locationy)))
  (bind _returnvalue_4 (Camera|GetCameraLocation _returnvalue))
  (bind _returnvalue_5 (Transformation|GetActorLocation _returnvalue_2))
  (bind (_returnvalue_6 _inrersectionpoint) (CallFunction|FindRaytoPlanePoint _returnvalue_4 _worlddirection "0.000000,0.000000,1.000000" _returnvalue_5))
  (if _returnvalue_6
    (Transformation|SetActorRotation _returnvalue_3 (Math|Rotator|MakeRotator 0.0 0.0 (.yaw (Math|Rotator|FindLookatRotation (Transformation|GetActorLocation _returnvalue_3) _inrersectionpoint))))))

(fn ConstructionScript)